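; BP_LearningBP is a procedural room generator that builds a tiled floor from a seeded random stream in the Construction Script.
; A NewSeed toggle rerolls the seed, then GenerateMap uses RoomMakeFloorArea to create a random-sized rectangle of grid tiles and record its extents.
; The loop covers RoomCount but only creates the first room.
; SpawnTiles adds each tile as a Floor mesh instance, positioned by Scale.
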(event Custom|Generate%20Map
  (for _index (range 0 (- (Variables|MapSettings|GetRoomCount) 1))
    (if (== _index 0)
      (bind (_floortiles __location _extents) (CallFunction|RoomMakeFloorArea (Variables|Default|GetPreviousLocation)))
      (Variables|Default|SetFloorTiles _floortiles)
      (Utilities|Map|Add (Variables|Default|GetRooms) __location _extents)))
  (CallFunction|SpawnTiles))

(fn ConstructionScript
  (Utilities|FlowControl|Sequence
    (:then_0
      ;[1 1 1] Gives Random Seed
      (if (Variables|EditorTools|GetNewSeed)
        (Variables|EditorTools|SetNewSeed false)
        (bind _output_get (Variables|MapSettings|SetSeed (Math|Random|RandomInteger 4184161)))
        (Math|Random|SetRandomStreamSeed (Variables|Default|GetStream) _output_get)))
    (:then_1
      ;[1 1 1] Manually update stream with seed
      (Math|Random|SetRandomStreamSeed (Variables|Default|GetStream) (Variables|MapSettings|GetSeed)))
    (:then_2
      (CallFunction|GenerateMap))))

(fn RoomMakeFloorArea
  (params (Location :type Int%20Vector%20Structure))
  (bind _roomsize_min (Variables|MapSettings|GetRoomSize_Min))
  (bind _roomsize_max (Variables|MapSettings|GetRoomSize_Max))
  (bind _stream (Variables|Default|GetStream))
  ;[1 1 1] Get Random X and Y extents and make array of floor tiles from X, Y added to root position
  (LocalVariables|SetRootLocation Location)
  (LocalVariables|SetOut_X (Math|Random|RandomIntegerinRangefromStream _roomsize_min _roomsize_max _stream))
  (LocalVariables|SetOut_Y (Math|Random|RandomIntegerinRangefromStream _roomsize_min _roomsize_max _stream))
  (for _index (range 0 (- (* (LocalVariables|GetOut_X) (LocalVariables|GetOut_Y)) 1))
    (Utilities|Array|Add (LocalVariables|GetTiles) (Utilities|Struct|MakeIntVector (+ (/ _index (LocalVariables|GetOut_Y)) (.X (Utilities|Struct|BreakIntVector (LocalVariables|GetRootLocation)))) (+ (Math|Integer|%(Integer) _index (LocalVariables|GetOut_Y)) (.Y (Utilities|Struct|BreakIntVector (LocalVariables|GetRootLocation)))) (.Z (Utilities|Struct|BreakIntVector (LocalVariables|GetRootLocation))))))
  (while (LocalVariables|GetWorking)
    (LocalVariables|SetWorking false)
    (LocalVariables|SetConnectedTiles (LocalVariables|GetTiles)))
  (for _array_element (LocalVariables|GetConnectedTiles)
    (Utilities|Array|Add (LocalVariables|GetExtents_X) (.X (Utilities|Struct|BreakIntVector _array_element)))
    (Utilities|Array|Add (LocalVariables|GetExtents_Y) (.Y (Utilities|Struct|BreakIntVector _array_element))))
  (return (LocalVariables|GetConnectedTiles) (LocalVariables|GetRootLocation) (Utilities|Struct|MakeIntVector (.MaxValue (Math|Integer|MaxOfIntArray (LocalVariables|GetExtents_X))) (.MaxValue (Math|Integer|MaxOfIntArray (LocalVariables|GetExtents_Y))))))

(fn SpawnTiles
  (for _array_element (Variables|Default|GetFloorTiles)
    (Components|InstancedStaticMesh|AddInstance (Variables|Default|GetFloor) (Math|Transform|MakeTransform (* (Math|Conversions|ToVector(Float) _array_element) (Variables|EditorTools|GetScale)) "0, 0, 0" "1,1,1"))))