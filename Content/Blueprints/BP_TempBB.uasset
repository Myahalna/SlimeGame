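; BP_TempBB is a construction-script actor that lays a desert tile grid sized to the bounds of all BP_DungeonGen actors, with Offset adding extra tiles.
; It moves itself to the bounds' minimum X less half the padding, while Y derives only from the padding, ignoring the bounds.
; Nested loops add instances at MeshScale spacing, randomly choosing Desert three times as often as DesertRocks.
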(event EventTick
  (params (DeltaSeconds :type Float%20%28single-precision%29)))

(fn ConstructionScript
  (bind _desert (Variables|Default|GetDesert))
  (bind _meshscale (Variables|Default|GetMeshScale))
  (bind _offset (Variables|Default|GetOffset))
  (bind _meshscale_2 (Variables|Default|GetMeshScale))
  (bind _outactors (Actor|GetAllActorsOfClass "/Game/Blueprints/BP_DungeonGen.BP_DungeonGen_C"))
  (bind (_center _boxextent) (Collision|GetActorArrayBounds _outactors true))
  (Transformation|SetActorLocation (Math|Vector|MakeVector (- (- (.x _center) (.x _boxextent)) (* (/ (Variables|Default|GetOffset) 2) (Variables|Default|GetMeshScale))) (- (* 0 (.y _center)) (* (/ _offset 2) _meshscale)) 0.0) false false)
  (for _index (range 0 (+ (* (Math|Float|Truncate (/ (.x _boxextent) _meshscale)) 2) _offset))
    (for _index_2 (range 0 (+ (* (Math|Float|Truncate (/ (.y _boxextent) _meshscale)) 2) _offset))
      (Components|InstancedStaticMesh|AddInstance (Utilities|Array|Get(acopy) (Utilities|Array|MakeArray _desert (Variables|Default|GetDesert_Rocks) _desert _desert) (Math|Random|RandomIntegerinRange 0 3)) (Math|Transform|MakeTransform (Math|Vector|MakeVector (* _index _meshscale_2) (* _index_2 _meshscale_2) 0.0) "0, 0, 0" "1,1,1")))))