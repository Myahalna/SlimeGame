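; BP_Statue is a ViewerArena display statue that shows a data-driven skeletal mesh in a non-playing animation pose, colored by element.
; The construction script reads mesh, animation and mask-set table from the DisplayMesh row, capping TextureMaskID at the last mask row.
; Each material slot gets a dynamic instance with its mask texture and four colors from the ElemColorData row named after the Element enum.
; The event graph is empty.
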(event EventBeginPlay)

(event Collision|EventActorBeginOverlap
  (params (OtherActor :type Actor%20Object%20Reference)))

(event EventTick
  (params (DeltaSeconds :type Float%20%28single-precision%29)))

(fn ConstructionScript
  (bind _displaymesh (Variables|Default|GetDisplayMesh))
  (bind _skeletalmesh (Variables|Default|GetSkeletalMesh))
  (bind (_datatable _rowname) (Utilities|Struct|BreakDataTableRowHandle _displaymesh))
  (Utilities|FlowControl|Sequence
    (:then_0
      (bind _returnvalue (Utilities|GetDataTableRow _datatable _rowname)
        (:then
          (Class|SkinnedMeshComponent|SetSkeletalMesh _skeletalmesh (.Meshs (Utilities|Struct|BreakStruct_StatueData _returnvalue)) true)
          (Variables|/Script/Engine.SkeletalMeshComponent|SetAnimationData _skeletalmesh (Utilities|Struct|MakeSingleAnimationPlayData (.Animations (Utilities|Struct|BreakStruct_StatueData _returnvalue)) true false 0.0))
          (bind _outrownames (DataTable|GetDataTableRowNames (.MaskSet (Utilities|Struct|BreakStruct_StatueData _returnvalue))))
          (if (> (- (Utilities|Array|Length _outrownames) 1) (Variables|Default|GetTextureMaskID))
            _
            (else
              (Variables|Default|SetTextureMaskID (- (Utilities|Array|Length _outrownames) 1))))
          (bind _returnvalue_2 (Utilities|GetDataTableRow (.MaskSet (Utilities|Struct|BreakStruct_StatueData _returnvalue)) (Utilities|Array|Get(acopy) _outrownames (Variables|Default|GetTextureMaskID)))
            (:then
              (for (_array_element _array_index) (Rendering|Material|GetMaterials (Variables|Default|GetSkeletalMesh))
                (bind _returnvalue_3 (Rendering|Material|CreateDynamicMaterialInstance _array_element "None" "None" :!class /Script/Engine.KismetMaterialLibrary))
                (Rendering|Material|SetMaterial (Variables|Default|GetSkeletalMesh) _array_index _returnvalue_3)
                (Rendering|Material|SetTextureParameterValue _returnvalue_3 "Mask" (Utilities|Array|Get(acopy) (.MaskTexture (Utilities|Struct|BreakStruct_PatternMask _returnvalue_2)) _array_index))
                (bind _returnvalue_4 (Utilities|GetDataTableRow "/Game/DataTable/ElemColorData.ElemColorData" (Utilities|String|StringToName (Utilities|String|EnumtoString (Variables|Default|GetElement))))
                  (:then
                    (Utilities|FlowControl|Sequence
                      (:then_0
                        (Rendering|Material|SetVectorParameterValue _returnvalue_3 "ColPrimary" (.Primary (Utilities|Struct|BreakElemStruct _returnvalue_4)) :!class /Script/Engine.MaterialInstanceDynamic))
                      (:then_1
                        (Rendering|Material|SetVectorParameterValue _returnvalue_3 "ColSecondary" (.Secondary (Utilities|Struct|BreakElemStruct _returnvalue_4)) :!class /Script/Engine.MaterialInstanceDynamic))
                      (:then_2
                        (Rendering|Material|SetVectorParameterValue _returnvalue_3 "ColTert1" (.Tertiary1 (Utilities|Struct|BreakElemStruct _returnvalue_4)) :!class /Script/Engine.MaterialInstanceDynamic))
                      (:then_3
                        (Rendering|Material|SetVectorParameterValue _returnvalue_3 "ColTert2" (.Tertiary2 (Utilities|Struct|BreakElemStruct _returnvalue_4)) :!class /Script/Engine.MaterialInstanceDynamic)))))))))))))